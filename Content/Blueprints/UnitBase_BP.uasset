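; UnitBase_BP is a unit pawn that can be selected, ordered to move and shown taking damage.
; Selection toggles the mesh material between selected and normal, and move orders pass the given location to AIMoveTo.
; The damage visual briefly swaps in a damage material, then always restores the normal one, even if the unit was selected.
; It holds no tick, overlap or damage calculation logic.
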(event `self.ToggleSelectedColor`
  (params (isSelected :type Boolean))
  (bind _meshcomponent (`self.MeshComponent`))
  (if isSelected
    (`PrimitiveComponent.SetMaterial` _meshcomponent 0 "/Game/Materials/Unit_Selected_Mat.Unit_Selected_Mat")
    (else
      (`PrimitiveComponent.SetMaterial` _meshcomponent 0 "/Game/Materials/Unit_Mat.Unit_Mat"))))

(event `self.MoveToLocation`
  (params (location :type "Vector Structure"))
  (`|AIMoveTo` self location null))

(event `self.TakeDamgeVisual`
  (bind _meshcomponent (`self.MeshComponent`))
  (`PrimitiveComponent.SetMaterial` _meshcomponent 0 "/Game/Materials/Unit_Damage_Mat.Unit_Damage_Mat")
  (`KismetSystemLibrary.Delay` 0.2)
  (`PrimitiveComponent.SetMaterial` _meshcomponent 0 "/Game/Materials/Unit_Mat.Unit_Mat"))

(fn `UserConstructionScript`)